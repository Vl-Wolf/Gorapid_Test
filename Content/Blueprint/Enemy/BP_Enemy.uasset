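; BP_Enemy is the Blueprint for an enemy character, handling its death, weapon animation events and entering cover.
; On death it plays the selected death montage, fires DeadEvent as playback starts and enables ragdoll on blend out.
; It caches ABP_Enemy at BeginPlay and forwards weapon fire and reload events to it.
; Entering cover sets a flag and crouches, while simple accessors expose whether the enemy can move or attack.
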(event `self.CharacterDead`
  (bind _returnvalue (`self.GetCharacterDeathMontage`))
  (`self.PlayDeathMontage` _returnvalue))

(event `PlayDeathMontage`
  (params (SelectedDead :type "AnimMontage Object Reference"))
  (`|PlayMontage` (`self.Mesh`) SelectedDead
    (:`then`
      (`self.DeadEvent`))
    (:`OnBlendOut`
      (`self.EnableRagdoll`))))

(event `self.ReceiveBeginPlay`
  (bind _asabp_enemy (cast `/Game/Characters/Enemy/ABP_Enemy` (`SkeletalMeshComponent.GetAnimInstance` (`self.Mesh`))))
  (set `self.AnimInstance` _asabp_enemy))

(event `self.WeaponFire_BP`
  (params (Anim :type "AnimMontage Object Reference"))
  (`/Game/Characters/Enemy/ABP_Enemy.Firing` (`self.AnimInstance`) Anim))

(event `self.WeaponReloadStart_BP`
  (params (Anim :type "AnimMontage Object Reference"))
  (`/Game/Characters/Enemy/ABP_Enemy.ReloadStart` (`self.AnimInstance`) Anim))

(event `self.WeaponReloadEnd_BP`
  (params (bIsSuccess :type Boolean))
  (`/Game/Characters/Enemy/ABP_Enemy.ReloadEnd` (`self.AnimInstance`) bIsSuccess))

(event `self.ReceiveTick`
  (params (DeltaSeconds :type "Float (single-precision)")))

(event `EnterCover`
  (set `self.bIsInCover` true)
  (`self.Crouch`))

(fn `CanAttack`
  (returns (bIsCanAttack :type Boolean))
  (return (`self.Can Attack`)))

(fn `CanMove`
  (returns (bIsCanMove :type Boolean))
  (return (`self.Can Move`)))

(fn `SetStateAttack`
  (params (bCanAttack :type Boolean))
  (set `self.Can Attack` bCanAttack))

(fn `SetStateMovement`
  (params (bCanMove :type Boolean))
  (set `self.Can Move` bCanMove))

(fn `UserConstructionScript`)
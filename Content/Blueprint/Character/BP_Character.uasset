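; Character Blueprint that plays weapon fire and reload animations through the third-person Animation Blueprint.
; BeginPlay caches the mesh's ABP_ThirdPerson instance.
; Weapon fire, reload start and reload end events route through multicast events, which hand the montage or success flag to that anim instance, apparently to replicate the animations.
; Debug leftovers include a key 1 death montage test and unconnected camera location prints.
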(event `self.ReceiveBeginPlay`
  (bind _asabp_third_person (cast `/Game/Characters/Player/Animations/ABP_ThirdPerson` (`SkeletalMeshComponent.GetAnimInstance` (`self.Mesh`))))
  (set `self.AnimInstance` _asabp_third_person))

(event `self.ReceiveTick`
  (params (DeltaSeconds :type "Float (single-precision)")))

(event `Key|One`
  (params (Key :type "Key Structure"))
  (:`Pressed`
    (`|PlayMontage` (`self.Mesh`) "/Game/Characters/Enemy/Animations/Death/Death_1_Montage.Death_1_Montage"
      (:`OnCompleted`
        (`KismetSystemLibrary.PrintString` "Hello")))))

(event `self.WeaponFire_BP`
  (params (Anim :type "AnimMontage Object Reference"))
  (`self.FireAnimStart_Multicast` Anim))

(event `self.WeaponReloadStart_BP`
  (params (Anim :type "AnimMontage Object Reference"))
  (`self.ReloadStart_Multicast` Anim))

(event `self.WeaponReloadEnd_BP`
  (params (bIsSuccess :type Boolean))
  (`self.ReloadEnd_Multicast` bIsSuccess))

(event `FireAnimStart_Multicast`
  (params (MontageToPlay :type "AnimMontage Object Reference"))
  (`/Game/Characters/Player/Animations/ABP_ThirdPerson.Firing` (`self.AnimInstance`) MontageToPlay))

(event `ReloadEnd_Multicast`
  (params (bIsSuccess :type Boolean))
  (`/Game/Characters/Player/Animations/ABP_ThirdPerson.ReloadEnd` (`self.AnimInstance`) bIsSuccess))

(event `ReloadStart_Multicast`
  (params (MontageToPlay :type "AnimMontage Object Reference"))
  (`/Game/Characters/Player/Animations/ABP_ThirdPerson.ReloadStart` (`self.AnimInstance`) MontageToPlay))

(fn `UserConstructionScript`)
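; Player controller that owns the in-game HUD and keeps it bound to the possessed BP_Character.
; On BeginPlay it creates BPW_InGameWidget for local players and wires its inventory and health sub-widgets to the character.
; Possess initializes the character's inventory from weapon slots stored in BP_PlayerState, then refreshes those widgets with them.
; UnPossess unbinds both widgets from the released pawn, falling back to the controlled pawn if none is valid.
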(event `self.ReceiveBeginPlay`
  (`/Engine/EditorBlueprintResources/ActorMacros.Switch Has Authority`
    (:`Authority`
      (if (`self.IsLocalPlayerController`)
        (bind _returnvalue (`|CreateWidget` "/Game/Widget/BPW_InGameWidget.BPW_InGameWidget_C" self :!label _label))
        (bind _output_get (set `self.InGameWidget` _returnvalue))
        (`UserWidget.AddToViewport` _output_get 0)
        (bind _asbp_character (cast `/Game/Blueprint/Character/BP_Character` (`GameplayStatics.GetPlayerPawn` 0)))
        (bind _bpw_inventorystats (`/Game/Widget/BPW_InGameWidget.BPW_InventoryStats` _output_get))
        (`/Game/Widget/BPW_InventoryStats.BindInventoryEvent` _bpw_inventorystats _asbp_character)
        (bind _inventorycomponent (`TTCharacter.InventoryComponent` _asbp_character))
        (`/Engine/EditorBlueprintResources/StandardMacros.IsValid` _inventorycomponent
          (:`Is Valid`
            (`/Game/Widget/BPW_InventoryStats.InitInventorySlots` _bpw_inventorystats (`TT_InventoryComponent.WeaponSlots` _inventorycomponent))
            (`/Game/Widget/BPW_CharacterHealth.InitWidget` (`/Game/Widget/BPW_InGameWidget.BPW_CharacterHealth` _output_get) _asbp_character)))))
    (:`Remote`
      (goto _label))))

(event `UnbindWidgetEvents`
  (params (Object :type "Object Object Reference"))
  (`self.UnbindWidgets` Object))

(event `InitWidget`
  (params (Weapons :type "Array of WeaponSlot Structure"))
  (bind _ingamewidget (`self.InGameWidget`))
  (bind _bpw_inventorystats (`/Game/Widget/BPW_InGameWidget.BPW_InventoryStats` _ingamewidget))
  (`/Engine/EditorBlueprintResources/StandardMacros.IsValid` _ingamewidget
    (:`Is Valid`
      (bind _asbp_character (cast `/Game/Blueprint/Character/BP_Character` (`self.K2_GetPawn`)))
      (`/Game/Widget/BPW_InventoryStats.BindInventoryEvent` _bpw_inventorystats _asbp_character)
      (`/Game/Widget/BPW_InventoryStats.InitInventorySlots` _bpw_inventorystats Weapons)
      (`/Game/Widget/BPW_CharacterHealth.InitWidget` (`/Game/Widget/BPW_InGameWidget.BPW_CharacterHealth` _ingamewidget) _asbp_character))))

(event `self.ReceivePossess`
  (params (PossessedPawn :type "Pawn Object Reference"))
  (bind _asbp_character (cast `/Game/Blueprint/Character/BP_Character` PossessedPawn))
  (bind _asbp_player_state (cast `/Game/Blueprint/Game/BP_PlayerState` (`self.PlayerState`)))
  (bind _inventorycomponent (`TTCharacter.InventoryComponent` _asbp_character))
  (`/Engine/EditorBlueprintResources/StandardMacros.IsValid` _inventorycomponent
    (:`Is Valid`
      (bind _weaponslot (`TT_PlayerState.WeaponSlot` _asbp_player_state))
      (`TT_InventoryComponent.InitInventory` _inventorycomponent _weaponslot)
      (`self.InitWidget` _weaponslot))))

(event `self.ReceiveUnPossess`
  (params (UnpossessedPawn :type "Pawn Object Reference"))
  (`self.UnbindWidgetEvents` UnpossessedPawn))

(fn `UnbindWidgets`
  (params (Object :type "Object Object Reference"))
  (locals (MyTarget :type "Object Object Reference"))
  (bind _ingamewidget (`self.InGameWidget`))
  (`/Engine/EditorBlueprintResources/StandardMacros.IsValid` Object
    (:`Is Valid`
      (set `local.MyTarget` Object))
    (:`Is Not Valid`
      (set `local.MyTarget` (`self.K2_GetPawn`))))
  (`/Engine/EditorBlueprintResources/StandardMacros.IsValid` (`self.InGameWidget`)
    (:`Is Valid`
      (bind _asbp_character (cast `/Game/Blueprint/Character/BP_Character` (`local.MyTarget`)))
      (`/Game/Widget/BPW_InventoryStats.UnbindAllEvents` (`/Game/Widget/BPW_InGameWidget.BPW_InventoryStats` _ingamewidget) _asbp_character)
      (`/Game/Widget/BPW_CharacterHealth.UnbindWidget` (`/Game/Widget/BPW_InGameWidget.BPW_CharacterHealth` _ingamewidget)))))

(fn `UserConstructionScript`)